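; BP_TileManager is a manager actor that generates a grid of BP_Tile actors when play begins.
; Nested loops over NbY (along world X) and NbX (along world Y) call SpawnBPTile at Spacing intervals, measured from the world origin.
; Each tile receives a reference to the manager on spawn, is added to the Tiles array and stores its index there.
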(event `self.ReceiveBeginPlay`
  (bind _spacing (`self.spacing`))
  ;[1 1 1] Y
  (for _index (range (+ (+ (`self.nbY`) -1) 1))
    ;[1 1 1] X
    (for _index_2 (range (+ (+ (`self.nbX`) -1) 1))
      (`self.SpawnBPTile` (* _index _spacing) (* _index_2 _spacing)))))

(fn `SpawnBPTile`
  (params (X :type Integer) (Y :type Integer))
  (bind _returnvalue (`|SpawnActorFromClass` "/Game/Blueprints/BP_Tile.BP_Tile_C" (`KismetMathLibrary.MakeTransform` (`KismetMathLibrary.MakeVector` (`KismetMathLibrary.Conv_IntToDouble` X) (`KismetMathLibrary.Conv_IntToDouble` Y))) "Undefined" "MultiplyWithRoot" null self null))
  (bind _returnvalue_2 (`KismetArrayLibrary.Array_Add` (`self.Tiles`) _returnvalue))
  (set `/Game/Blueprints/BP_Tile.IndexInManager` _returnvalue_2 _returnvalue))

(fn `UserConstructionScript`)